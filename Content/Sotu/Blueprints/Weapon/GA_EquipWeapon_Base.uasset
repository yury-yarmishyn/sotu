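; Base gameplay ability that equips the owner's current weapon and plays the matching equip animation.
; Setup fetches the weapon component, its current weapon data and the weapon handler mesh through interface calls, ending the ability if any is invalid.
; On commit, it applies each data entry's mesh, transform and anim class to handler child components matched by socket.
; It then plays a standing or crouched montage, chosen by gameplay tag, and ends with it.
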(event `self.K2_ActivateAbility`
  (bind _result (`self.SetupAbilityData`))
  (if _result
    (`self.K2_CommitAbility`)
    (else
      (`self.K2_EndAbility`))))

(event `self.K2_CommitExecute`
  (`self.AttachWeaponToHandler`)
  (`self.PlayAnimations`))

(event `PlayAnimations`
  (bind _weapondata (`self.WeaponData`))
  (bind _weaponhandler (`self.WeaponHandler`))
  (if (not (`GameplayTagAssetInterface.HasAnyMatchingGameplayTags` (`self.GetAbilitySystemComponentFromActorInfo`) (`BlueprintGameplayTagLibrary.MakeLiteralGameplayTagContainer` (struct :`GameplayTags` (struct :`(TagName` "State.Movement.Crouching") :`(TagName` "State.Movement.Sliding"))))))
    (`|PlayMontage` _weaponhandler (`/Game/Sotu/Blueprints/Weapon/BP_WeaponData.HandlerEquipMontage` _weapondata)
      (:`OnCompleted`
        _)
      (:`OnBlendOut`
        _)
      (:`OnInterrupted`
        _))
    (else
      (`|PlayMontage` _weaponhandler (`/Game/Sotu/Blueprints/Weapon/BP_WeaponData.HandlerEquipMontage_Crouch` _weapondata)
        (:`OnCompleted`
          _)
        (:`OnBlendOut`
          _)
        (:`OnInterrupted`
          _))))
  (`self.K2_EndAbility`))

(fn `AttachWeaponToHandler`
  (bind _output_get (set `/Game/Sotu/Blueprints/Weapon/BPC_WeaponComponent.CurrentWeaponData` (`self.WeaponData`) (`self.Weapon Component`)))
  (for _array_element (`/Game/Sotu/Blueprints/Weapon/BP_WeaponData.WeaponData` _output_get)
    (for _array_element_2 (`SceneComponent.GetChildrenComponents` (`self.WeaponHandler`) false)
      (bind (_weaponmesh _weapontransform _sockettoattach _animinstance) (break `/Game/Sotu/Blueprints/Weapon/S_EquipWeaponData` _array_element))
      (if (== (`SceneComponent.GetAttachSocketName` _array_element_2) _sockettoattach)
        (bind _asskeletal_mesh_component (cast `SkeletalMeshComponent` _array_element_2))
        (`SkeletalMeshComponent.SetSkeletalMeshAsset` _asskeletal_mesh_component _weaponmesh)
        (`SceneComponent.K2_SetRelativeTransform` _asskeletal_mesh_component _weapontransform false false)
        (`SkeletalMeshComponent.SetAnimInstanceClass` _asskeletal_mesh_component _animinstance)))))

(fn `SetupAbilityData`
  (returns (Result :type Boolean))
  (bind _weaponcomponent (message `/Game/Sotu/Blueprints/Weapon/BPI_WeaponInrerface.GetWeaponComponent` (`self.GetOwningActorFromActorInfo`)))
  (`/Engine/EditorBlueprintResources/StandardMacros.IsValid` _weaponcomponent
    (:`Is Valid`
      (bind _output_get (set `self.Weapon Component` _weaponcomponent))
      (bind _currentweapondata (`/Game/Sotu/Blueprints/Weapon/BPC_WeaponComponent.CurrentWeaponData` _output_get))
      (`/Engine/EditorBlueprintResources/StandardMacros.IsValid` _currentweapondata
        (:`Is Valid`
          (set `self.WeaponData` _currentweapondata)
          (bind _weaponhandler (message `/Game/Sotu/Blueprints/Weapon/BPI_WeaponInrerface.GetWeaponHandler` (`self.GetOwningActorFromActorInfo`)))
          (bind _output_get_2 (set `self.WeaponHandler` _weaponhandler))
          (return (`KismetSystemLibrary.IsValid` _output_get_2)))
        (:`Is Not Valid`
          (return false))))
    (:`Is Not Valid`
      (return false))))