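; Base gameplay ability for unequipping the owner's current weapon by clearing its visuals.
; On activation it fetches the weapon component, current weapon data and weapon handler via interface messages on the owning actor, ending if any is invalid.
; On commit it resets the mesh, relative transform and anim class on the handler's child skeletal meshes, leaving the components in place.
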(event `self.K2_ActivateAbility`
  (bind _result (`self.SetupAbilityData`))
  (if _result
    (`self.K2_CommitAbility`)
    (else
      (`self.K2_EndAbility`))))

(event `self.K2_CommitExecute`
  (`self.DetachWeaponFromHandler`))

(fn `DetachWeaponFromHandler`
  (for _array_element (`SceneComponent.GetChildrenComponents` (`self.WeaponHandler`) false)
    (bind _asskeletal_mesh_component (cast `SkeletalMeshComponent` _array_element))
    (`SkeletalMeshComponent.SetSkeletalMeshAsset` _asskeletal_mesh_component null)
    (`SceneComponent.K2_SetRelativeTransform` _asskeletal_mesh_component (`KismetMathLibrary.MakeTransform` (0.0 0.0 0.0)) false false)
    (`SkeletalMeshComponent.SetAnimInstanceClass` _asskeletal_mesh_component null)))

(fn `SetupAbilityData`
  (returns (Result :type Boolean))
  (bind _weaponcomponent (message `/Game/Sotu/Blueprints/Weapon/BPI_WeaponInrerface.GetWeaponComponent` (`self.GetOwningActorFromActorInfo`)))
  (`/Engine/EditorBlueprintResources/StandardMacros.IsValid` _weaponcomponent
    (:`Is Valid`
      (bind _output_get (set `self.WeaponComponent` _weaponcomponent))
      (bind _currentweapondata (`/Game/Sotu/Blueprints/Weapon/BPC_WeaponComponent.CurrentWeaponData` _output_get))
      (`/Engine/EditorBlueprintResources/StandardMacros.IsValid` _currentweapondata
        (:`Is Valid`
          (set `self.WeaponData` _currentweapondata)
          (bind _weaponhandler (message `/Game/Sotu/Blueprints/Weapon/BPI_WeaponInrerface.GetWeaponHandler` (`self.GetOwningActorFromActorInfo`)))
          (bind _output_get_2 (set `self.WeaponHandler` _weaponhandler))
          (return (`KismetSystemLibrary.IsValid` _output_get_2)))
        (:`Is Not Valid`
          (return false))))
    (:`Is Not Valid`
      (return false))))