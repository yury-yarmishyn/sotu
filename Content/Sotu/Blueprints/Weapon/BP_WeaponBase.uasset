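; BP_WeaponBase is a weapon base actor with left-hand and right-hand weapon components that can be switched in and out of use.
; The construction script sets each hand component's relative transform from WeaponData.
; SetinUse stores the InUse flag and toggles collision, visibility and tick together, so an unused weapon is hidden and inactive without being destroyed.
; GetInUse exposes the current flag.
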(event `/Game/Sotu/Blueprints/ObjectPool/BPI_ObjectPool.SetInUse`
  (params (`bInUse?` :type Boolean))
  (bind _output_get (set `self.bInUse?` `bInUse?`))
  (`self.SetActorEnableCollision` _output_get)
  (`self.SetActorHiddenInGame` (not _output_get))
  (`self.SetActorTickEnabled` _output_get))

(fn `GetInUse`
  (returns (`bInUse?` :type Boolean))
  (return (`self.bInUse?`)))

(fn `UserConstructionScript`
  (bind _weapondata (`self.WeaponData`))
  (`SceneComponent.K2_SetRelativeTransform` (`self.LeftHandWeapon`) (`/Game/Sotu/Blueprints/Weapon/BP_WeaponData.LeftHandWeaponTransform` _weapondata) false false)
  (`SceneComponent.K2_SetRelativeTransform` (`self.RightHandWeapon`) (`/Game/Sotu/Blueprints/Weapon/BP_WeaponData.RightHandWeaponTransform` _weapondata) false false))