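; Base gameplay ability that equips a weapon by spawning its actor and attaching it to the owner's weapon handler mesh.
; Activation fetches WeaponData and the handler through interface messages on the owning actor, ending early if setup fails.
; On commit, it spawns the weapon class, attaches left and right hand parts to data-defined sockets, and plays a standing or crouching handler montage based on the crouch gameplay tag.
; The ability ends when the montage completes, blends out or is interrupted.
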(event `self.K2_ActivateAbility`
  (bind _result (`self.SetupAbilityData`))
  (if _result
    (`self.K2_CommitAbility`)
    (else
      (`self.K2_EndAbility`))))

(event `self.K2_CommitExecute`
  (`self.SpawnAndSetWeapon`)
  (`self.AttachWeaponToHandler`)
  (`self.PlayAnimations`))

(event `PlayAnimations`
  (bind _weaponhandler (`self.WeaponHandler`))
  (bind _weapondata (`self.WeaponData`))
  (if (not (`GameplayTagAssetInterface.HasAnyMatchingGameplayTags` (`self.GetAbilitySystemComponentFromActorInfo`) (`BlueprintGameplayTagLibrary.MakeLiteralGameplayTagContainer` (struct :`GameplayTags` (struct :`(TagName` "State.Movement.Crouching") :`(TagName` "State.Movement.Sliding"))))))
    (`|PlayMontage` _weaponhandler (`.WeaponHandler_11_42A32D954951EBA57D897DB674EFE13F` (break `/Game/Sotu/Blueprints/Weapon/S_WeaponAnimMontages` (`/Game/Sotu/Blueprints/Weapon/BP_WeaponData.EquipMontages` _weapondata)))
      (:`OnCompleted`
        _)
      (:`OnBlendOut`
        _)
      (:`OnInterrupted`
        _))
    (else
      (`|PlayMontage` _weaponhandler (`.WeaponHandler_11_42A32D954951EBA57D897DB674EFE13F` (break `/Game/Sotu/Blueprints/Weapon/S_WeaponAnimMontages` (`/Game/Sotu/Blueprints/Weapon/BP_WeaponData.EquipMontages_Crouch` _weapondata)))
        (:`OnCompleted`
          _)
        (:`OnBlendOut`
          _)
        (:`OnInterrupted`
          _))))
  (`self.K2_EndAbility`))

(fn `AttachWeaponToHandler`
  (bind _weapondata (`self.WeaponData`))
  (bind _weaponhandler (`self.WeaponHandler`))
  (bind _weaponref (`self.WeaponREF`))
  (`Actor.K2_AttachToComponent` _weaponref _weaponhandler "None" "KeepRelative" "KeepRelative" "KeepRelative" true)
  (`SceneComponent.K2_AttachToComponent` (`/Game/Sotu/Blueprints/Weapon/BP_WeaponBase.LeftHandWeapon` _weaponref) _weaponhandler (`/Game/Sotu/Blueprints/Weapon/BP_WeaponData.LeftHandSocketName` _weapondata) "KeepRelative" "KeepRelative" "KeepRelative" true)
  (`SceneComponent.K2_AttachToComponent` (`/Game/Sotu/Blueprints/Weapon/BP_WeaponBase.RightHandWeapon` _weaponref) _weaponhandler (`/Game/Sotu/Blueprints/Weapon/BP_WeaponData.RightHandSocketName` _weapondata) "KeepRelative" "KeepRelative" "KeepRelative" true))

(fn `SetupAbilityData`
  (returns (Result :type Boolean))
  (bind _weaponcomponent (message `/Game/Sotu/Blueprints/Weapon/BPI_WeaponInrerface.GetWeaponComponent` (`self.GetOwningActorFromActorInfo`)))
  (`/Engine/EditorBlueprintResources/StandardMacros.IsValid` _weaponcomponent
    (:`Is Valid`
      (set `self.WeaponData` (`/Game/Sotu/Blueprints/Weapon/BPC_WeaponComponent.WeaponData` _weaponcomponent))
      (bind _weaponhandler (message `/Game/Sotu/Blueprints/Weapon/BPI_WeaponInrerface.GetWeaponHandler` (`self.GetOwningActorFromActorInfo`)))
      (bind _output_get (set `self.WeaponHandler` _weaponhandler))
      (return (`KismetSystemLibrary.IsValid` _output_get)))
    (:`Is Not Valid`
      (return false))))

(fn `SpawnAndSetWeapon`
  (bind _returnvalue (`|SpawnActorFromClass` (`/Game/Sotu/Blueprints/Weapon/BP_WeaponData.WeaponClass` (`self.WeaponData`)) (`KismetMathLibrary.MakeTransform` (0.0 0.0 0.0)) "Undefined" "MultiplyWithRoot" null null))
  (set `self.WeaponREF` _returnvalue)
  (return))