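; Gameplay ability that equips a weapon on its owner when an Ability.Weapon.Equip gameplay event arrives.
; It reads the BP_WeaponData payload, spawns that weapon class and passes it to the owner's weapon component to attach to the handler.
; It then plays a standing or crouching blades equip montage on the handler mesh, chosen by the crouching tag, and ends when the montage completes, blends out or is interrupted.
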(event `self.K2_ActivateAbility`
  (bind (_asynctaskproxy _payload) (`AbilityAsync_WaitGameplayEvent.WaitGameplayEventToActor` (`self.GetOwningActorFromActorInfo`) (struct :`TagName` "Ability.Weapon.Equip"))
    (:`EventReceived`
      (bind _asbp_weapon_data (cast `/Game/Sotu/Blueprints/Weapon/BP_WeaponData` (`.OptionalObject` (break `GameplayEventData` _payload))))
      (bind _returnvalue (`|SpawnActorFromClass` (`/Game/Sotu/Blueprints/Weapon/BP_WeaponData.WeaponClass` _asbp_weapon_data) (`KismetMathLibrary.MakeTransform` (0.0 0.0 0.0)) "Undefined" "MultiplyWithRoot" null null))
      (bind _output_get (set `self.CurrentWeapon` _returnvalue))
      (bind _weaponcomponent (message `/Game/Sotu/Blueprints/Weapon/BPI_WeaponInrerface.GetWeaponComponent` (`self.GetOwningActorFromActorInfo`)))
      (`/Game/Sotu/Blueprints/Weapon/BPC_WeaponComponent.AttachWeaponToHandler` _weaponcomponent _output_get)
      (if (not (`GameplayTagAssetInterface.HasAnyMatchingGameplayTags` (`self.GetAbilitySystemComponentFromActorInfo`) (`BlueprintGameplayTagLibrary.MakeLiteralGameplayTagContainer` (struct :`GameplayTags` (struct :`(TagName` "State.Movement.Crouching") :`(TagName` "State.Movement.Sliding"))))))
        (bind _weaponhandler (`/Game/Sotu/Blueprints/Weapon/BPC_WeaponComponent.WeaponHandler` _weaponcomponent))
        (`|PlayMontage` _weaponhandler "/Game/Sotu/Animations/AM_Player_Blades_Equip.AM_Player_Blades_Equip"
          (:`OnCompleted`
            _)
          (:`OnBlendOut`
            _)
          (:`OnInterrupted`
            _))
        (else
          (`|PlayMontage` _weaponhandler "/Game/Sotu/Animations/AM_Player_Blades_Equip_Crouch.AM_Player_Blades_Equip_Crouch"
            (:`OnCompleted`
              _)
            (:`OnBlendOut`
              _)
            (:`OnInterrupted`
              _))))
      (`self.K2_EndAbility`))))