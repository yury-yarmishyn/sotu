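; Blueprint function library with helpers that add or remove a single loose gameplay tag on an actor.
; Both wrap the tag in a container and pass it, with a replication flag, to the plural loose-tag functions.
; Add first queries the actor's Ability System Component through an interface message and skips tags already present, avoiding stacked counts.
; Remove passes straight through without a check.
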(fn `AddLooseGameplayTag`
  (params (Actor :type "Actor Object Reference") (GameplayTag :type "GameplayTag Structure") (bShouldReplicate :type Boolean))
  (returns (ReturnValue :type Boolean))
  (bind _returnvalue (`BlueprintGameplayTagLibrary.MakeGameplayTagContainerFromTag` GameplayTag))
  (bind _abilitysystemcomponent (message `/Game/Sotu/Blueprints/GAS/BPI_AbilitySystemInterface.GetAbilitySystemComponent` Actor))
  (if (not (`GameplayTagAssetInterface.HasAllMatchingGameplayTags` _abilitysystemcomponent _returnvalue))
    (bind _returnvalue_2 (`AbilitySystemBlueprintLibrary.AddLooseGameplayTags` Actor _returnvalue bShouldReplicate))
    (return _returnvalue_2)))

(fn `RemoveLooseGameplayTag`
  (params (Actor :type "Actor Object Reference") (GameplayTag :type "GameplayTag Structure") (bShouldReplicate :type Boolean))
  (returns (ReturnValue :type Boolean))
  (bind _returnvalue (`AbilitySystemBlueprintLibrary.RemoveLooseGameplayTags` Actor (`BlueprintGameplayTagLibrary.MakeGameplayTagContainerFromTag` GameplayTag) bShouldReplicate))
  (return _returnvalue))