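; BPC_CombatComponent is an actor component that bridges its owner's combat actions to the Gameplay Ability System.
; On BeginPlay it fetches the owner's ability system component and weapons through interface messages, then grants each configured combat ability with an input ID derived from the current ability count.
; Attack and EquipWeapon check the passed ability class is valid, then try to activate it by class with remote activation allowed.
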(event `self.ReceiveBeginPlay`
  (`self.SetupCombatComponent`))

(fn `Attack`
  (params (AttackAbilityClass :type "/Game/Sotu/Blueprints/Combat/GA_Attack_Base Class Reference"))
  (if (`KismetSystemLibrary.IsValidClass` AttackAbilityClass)
    (`AbilitySystemComponent.TryActivateAbilityByClass` (`self.AbilitySystemComponent`) AttackAbilityClass true)))

(fn `EquipWeapon`
  (params (WeaponAbility :type "/Game/Sotu/Blueprints/Combat/Equip/GA_Equip_Base Class Reference"))
  (if (`KismetSystemLibrary.IsValidClass` WeaponAbility)
    (`AbilitySystemComponent.TryActivateAbilityByClass` (`self.AbilitySystemComponent`) WeaponAbility true)))

(fn `GetAbilitySystemComponent`
  (bind _abilitysystemcomponent (message `/Game/Sotu/Blueprints/GAS/BPI_AbilitySystemInterface.GetAbilitySystemComponent` (`self.GetOwner`)))
  (set `self.AbilitySystemComponent` _abilitysystemcomponent))

(fn `GetCombatUtilities`
  (bind _weapons (message `/Game/Sotu/Blueprints/Combat/BPI_CombatInterface.GetWeapons` (`self.GetOwner`)))
  (set `self.Weapons` _weapons))

(fn `SetupCombatAbilities`
  (bind _abilitysystemcomponent (`self.AbilitySystemComponent`))
  (for _array_element (`self.CombatAbilties`)
    (bind _outabilityhandles (`AbilitySystemComponent.GetAllAbilities` _abilitysystemcomponent))
    (bind _result (`/Engine/EditorBlueprintResources/StandardMacros.IncrementInt` (`KismetArrayLibrary.Array_Length` _outabilityhandles))
      (:`  `
        (`AbilitySystemComponent.K2_GiveAbility` _abilitysystemcomponent _array_element 0 _result)))))

(fn `SetupCombatComponent`
  (`self.GetAbilitySystemComponent`)
  (`self.GetCombatUtilities`)
  (`self.SetupCombatAbilities`))