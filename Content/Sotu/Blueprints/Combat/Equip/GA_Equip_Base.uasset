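; Base Gameplay Ability for equipping weapons, applying a weapon data asset's meshes to the owner's weapon mesh components.
; On activation it fetches the owner's socket-keyed component map and commits only if WeaponData is valid.
; Commit sets mesh, transform and anim class on matching sockets, then plays a standing or crouched equip montage based on the crouching tag.
; Ending the ability calls UnequipWeapon, an empty event here.
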(event `self.K2_ActivateAbility`
  (`self.SetupAbilityData`)
  (`/Engine/EditorBlueprintResources/StandardMacros.IsValid` (`self.WeaponData`)
    (:`Is Valid`
      (`self.K2_CommitAbility`))
    (:`Is Not Valid`
      (`self.K2_EndAbility`))))

(event `self.K2_CommitExecute`
  (`self.EquipWeapon`)
  (`self.PlayAnimations`))

(event `PlayAnimations`
  (bind _weapondata (`self.WeaponData`))
  (bind _value (`BlueprintMapLibrary.Map_Find` (`self.Weapons`)))
  (if (not (`GameplayTagAssetInterface.HasAnyMatchingGameplayTags` (`self.GetAbilitySystemComponentFromActorInfo`) (`BlueprintGameplayTagLibrary.MakeLiteralGameplayTagContainer` (struct :`GameplayTags` (struct :`(TagName` "State.Movement.Crouching") :`(TagName` "State.Movement.Sliding"))))))
    (`|PlayMontage` _value (`/Game/Sotu/Blueprints/Combat/Equip/BP_WeaponData.HandlerEquipMontage` _weapondata))
    (else
      (`|PlayMontage` _value (`/Game/Sotu/Blueprints/Combat/Equip/BP_WeaponData.HandlerEquipMontage_Crouch` _weapondata)))))

(event `UnequipWeapon`)

(event `self.K2_OnEndAbility`
  (params (bWasCancelled :type Boolean))
  (`self.UnequipWeapon`))

(event `EquipWeapon`
  (for _array_element (`/Game/Sotu/Blueprints/Combat/Equip/BP_WeaponData.WeaponData` (`self.WeaponData`))
    (bind (_keypin _valuepin) (`|MapForEach` (`self.Weapons`))
      (:`then`
        (bind (_weaponmesh _weapontransform _sockettoattach _animinstance) (break `/Game/Sotu/Blueprints/Combat/S_EquipWeaponData` _array_element))
        (if (== _keypin _sockettoattach)
          (`SkeletalMeshComponent.SetSkeletalMeshAsset` _valuepin _weaponmesh)
          (`SceneComponent.K2_SetRelativeTransform` _valuepin _weapontransform false false)
          (`SkeletalMeshComponent.SetAnimInstanceClass` _valuepin _animinstance))))))

(fn `SetupAbilityData`
  (bind _weapons (message `/Game/Sotu/Blueprints/Combat/BPI_CombatInterface.GetWeapons` (`self.GetOwningActorFromActorInfo`)))
  (set `self.Weapons` _weapons))