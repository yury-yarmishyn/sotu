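; Base Gameplay Ability for attacks that plays montages on the owning actor's weapon meshes.
; On activation it fetches the weapon map through an interface message, then plays each attack entry's montages on the meshes matched by key.
; A montage Notify Begin ends the ability.
; A helper, not called here, builds a Gameplay Effect spec with SetByCaller magnitudes and applies it to the owner's own Ability System Component.
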(event `self.K2_ActivateAbility`
  (`self.SetupAbilityData`)
  (for _array_element (`self.AttackData`)
    (`self.PlayAnimations` (`/Game/Sotu/Blueprints/Combat/BP_AttackData.AttackMontages` _array_element))))

(event `PlayAnimations`
  (params (AnimMontages :type "Map of Name to AnimMontage Object Reference"))
  (bind (_keypin _valuepin) (`|MapForEach` AnimMontages)
    (:`then`
      (`|PlayMontage` (`BlueprintMapLibrary.Map_Find` (`self.Weapons`) _keypin) _valuepin
        (:`OnNotifyBegin`
          (`self.K2_EndAbility`))))))

(fn `ApplyAttackEffect`
  (params (AttackEffect :type "/Game/Sotu/Blueprints/Combat/S_AttackEffectData Structure"))
  (locals (EffectSpec :type "GameplayEffectSpecHandle Structure"))
  (bind (_gameplayeffect _magnitudedata) (break `/Game/Sotu/Blueprints/Combat/S_AttackEffectData` AttackEffect))
  (bind _effectspec (`local.EffectSpec`))
  (bind _returnvalue (`AbilitySystemBlueprintLibrary.MakeSpecHandleByClass` _gameplayeffect null (`self.GetOwningActorFromActorInfo`)))
  (set `local.EffectSpec` _returnvalue)
  (bind (_keypin _valuepin) (`|MapForEach` _magnitudedata)
    (:`then`
      (`AbilitySystemBlueprintLibrary.AssignTagSetByCallerMagnitude` _effectspec _keypin _valuepin))
    (:`CompletedPin`
      (`AbilitySystemComponent.BP_ApplyGameplayEffectSpecToSelf` (`self.GetAbilitySystemComponentFromActorInfo`) _effectspec))))

(fn `SetupAbilityData`
  (bind _weapons (message `/Game/Sotu/Blueprints/Combat/BPI_CombatInterface.GetWeapons` (`self.GetOwningActorFromActorInfo`)))
  (set `self.Weapons` _weapons))