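; Base character Blueprint with an Ability System Component, providing start/end events for sprint, slide, crouch and jump.
; These events adjust movement speed and friction; timelines resize the capsule and ease slide speed, holding maximum speed on downhill slopes.
; Looping timers and movement callbacks maintain gameplay tags for sliding, airborne and blocked standing, the last gating capsule regrowth via sphere traces.
; Ending a slide attempts the crouch ability.
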(event `self.ReceiveBeginPlay`
  (add `SotuAbilitySystemComponent.OnAttributeChanged` (`self.BPC_AbilitySystemComponent`) (delegate `Event_OnAttributeChanged`))
  (`self.CapsuleSetup`)
  (`self.CharacterMovementSetup`))

(event `self.K2_OnMovementModeChanged`
  (params (PrevMovementMode :type "EMovementMode Enum" :default "MOVE_None") (NewMovementMode :type "EMovementMode Enum" :default "MOVE_None") (PrevCustomMode :type Byte) (NewCustomMode :type Byte))
  (if (and (`|EnumEquality` PrevMovementMode "MOVE_Walking") (`|EnumEquality` NewMovementMode "MOVE_Falling"))
    (`/Game/Sotu/Blueprints/BPFL_Sotu.AddLooseGameplayTag` self (`self.ContextInAirTag`))))

(event `Event_OnAttributeChanged`
  (params (Attribute :type "GameplayAttribute Structure") (OldValue :type "Float (single-precision)") (NewValue :type "Float (single-precision)")))

(event `self.OnLanded`
  (params (Hit :type "HitResult Structure (by ref)"))
  (`/Game/Sotu/Blueprints/BPFL_Sotu.RemoveLooseGameplayTag` self (`self.ContextInAirTag`)))

(event `/Game/Sotu/Blueprints/GAS/BPI_Movement.StartSprint`
  (set `CharacterMovementComponent.MaxWalkSpeed` (`self.MaxSprintSpeed`) (`self.CharacterMovement`)))

(event `/Game/Sotu/Blueprints/GAS/BPI_Movement.StartSlide`
  (bind _charactermovement (`self.CharacterMovement`))
  (set `CharacterMovementComponent.MaxWalkSpeed` (`self.MaxSlideSpeed`) _charactermovement)
  (set `CharacterMovementComponent.BrakingDecelerationWalking` (`self.SlideBrakingDecelerationWalking`) _charactermovement)
  (set `CharacterMovementComponent.GroundFriction` (`self.SlideGroundFriction`) _charactermovement)
  (`self.StartSlide_Anim`))

(event `/Game/Sotu/Blueprints/GAS/BPI_Movement.StartJump`
  (`self.Jump`))

(event `/Game/Sotu/Blueprints/GAS/BPI_Movement.StartCrouch`
  (set `CharacterMovementComponent.MaxWalkSpeed` (`self.MaxCrouchSpeed`) (`self.CharacterMovement`))
  (`self.StartCrouch_Anim`))

(event `/Game/Sotu/Blueprints/GAS/BPI_Movement.EndSlide`
  (bind _charactermovement (`self.CharacterMovement`))
  (set `CharacterMovementComponent.MaxWalkSpeed` (`self.MaxWalkSpeed`) _charactermovement)
  (set `CharacterMovementComponent.BrakingDecelerationWalking` (`self.BrakingDecelerationWalking`) _charactermovement)
  (set `CharacterMovementComponent.GroundFriction` (`self.GroundFriction`) _charactermovement)
  (`self.EndSlide_Anim`)
  (`AbilitySystemComponent.TryActivateAbilityByClass` (`self.BPC_AbilitySystemComponent`) "/Game/Sotu/Blueprints/GAS/GameplayAbilities/GA_Crouch.GA_Crouch_C" true))

(event `/Game/Sotu/Blueprints/GAS/BPI_Movement.EndJump`
  (`self.StopJumping`))

(event `/Game/Sotu/Blueprints/GAS/BPI_Movement.EndSprint`
  (set `CharacterMovementComponent.MaxWalkSpeed` (`self.MaxWalkSpeed`) (`self.CharacterMovement`)))

(event `/Game/Sotu/Blueprints/GAS/BPI_Movement.EndCrouch`
  (set `CharacterMovementComponent.MaxWalkSpeed` (`self.MaxWalkSpeed`) (`self.CharacterMovement`))
  (`self.EndCrouch_Anim`))

(event `StartCrouch_Anim`
  (bind _crouchtimeline (`self.CrouchTimeline`))
  (`TimelineComponent.SetPlayRate` _crouchtimeline (/ (`TimelineComponent.GetTimelineLength` _crouchtimeline) (`self.CrouchDuration`)))
  (`self.StartTimer_CanStand`)
  (bind (_direction _alpha) (`Timeline|CrouchTimeline` :!label _label)
    (:`Update`
      (switch `ETimelineDirection` _direction
        (:`Forward`
          (`CapsuleComponent.SetCapsuleHalfHeight` (`self.CapsuleComponent`) (`KismetMathLibrary.Lerp` (`self.CapsuleHalfHeight`) (`self.CrouchHalfHeight`) _alpha) true :!label _label_2))
        (:`Backward`
          (if (not (`GameplayTagAssetInterface.HasMatchingGameplayTag` (`self.BPC_AbilitySystemComponent`) (`self.ContextCannotStandTag`)))
            (goto _label_2)))))))

(event `StartSlide_Anim`
  (bind _result (`self.IsInfiniteSlide`))
  (bind _charactermovement (`self.CharacterMovement`))
  (bind _maxslidespeed (`self.MaxSlideSpeed`))
  (`TimelineComponent.SetPlayRate` (`self.SlideTimeline`) (/ (`TimelineComponent.GetTimelineLength` (`self.SlideTimeline`)) (`self.SlideDuration`)))
  (`self.StartCrouch_Anim`)
  (`self.StartTimer_StateSlide`)
  (bind (_direction _alpha) (`Timeline|SlideTimeline` :!via `PlayFromStart` :!label _label_3)
    (:`Update`
      (`TimelineComponent.SetLooping` (`self.SlideTimeline`) _result)
      (if (not _result)
        (set `CharacterMovementComponent.MaxWalkSpeed` (`KismetMathLibrary.Lerp` (`self.MaxCrouchSpeed`) _maxslidespeed _alpha) _charactermovement)
        (else
          (set `CharacterMovementComponent.MaxWalkSpeed` _maxslidespeed _charactermovement))))))

(event `EndCrouch_Anim`
  (`self.EndTimer_CanStand`)
  (goto _label :!via `Reverse`))

(event `EndSlide_Anim`
  (`self.EndCrouch_Anim`)
  (`self.EndTimer_StateSlide`)
  (goto _label_3 :!via `Stop`))

(event `StartTimer_StateSlide`
  (bind _returnvalue (`KismetSystemLibrary.K2_SetTimerDelegate` (delegate `Event_StateSlide`) (`GameplayStatics.GetWorldDeltaSeconds`) true))
  (set `self.StateSlideTimerHandle` _returnvalue))

(event `StartTimer_CanStand`
  (bind _returnvalue (`KismetSystemLibrary.K2_SetTimerDelegate` (delegate `Event_CanStand`) (`GameplayStatics.GetWorldDeltaSeconds`) true true))
  (set `self.CanStandTimerHandle` _returnvalue))

(event `Event_StateSlide`
  (bind _stateslidetag (`self.StateSlideTag`))
  (if (>= (`KismetMathLibrary.VSize` (`self.GetVelocity`)) (`self.MaxCrouchSpeed`))
    (`/Game/Sotu/Blueprints/BPFL_Sotu.AddLooseGameplayTag` self _stateslidetag)
    (else
      (`/Game/Sotu/Blueprints/BPFL_Sotu.RemoveLooseGameplayTag` self _stateslidetag))))

(event `Event_CanStand`
  (bind _contextcannotstandtag (`self.ContextCannotStandTag`))
  (if (`self.CanStand`)
    (`/Game/Sotu/Blueprints/BPFL_Sotu.RemoveLooseGameplayTag` self _contextcannotstandtag)
    (else
      (`/Game/Sotu/Blueprints/BPFL_Sotu.AddLooseGameplayTag` self _contextcannotstandtag))))

(event `EndTimer_StateSlide`
  (`KismetSystemLibrary.K2_ClearAndInvalidateTimerHandle` (`self.StateSlideTimerHandle`)))

(event `EndTimer_CanStand`
  (`KismetSystemLibrary.K2_ClearAndInvalidateTimerHandle` (`self.CanStandTimerHandle`)))

(fn `CanStand`
  (returns (Result :type Boolean))
  (locals (CapsuleTiltAngle :type "Float (double-precision)" :default 45.0))
  (bind _returnvalue (`self.K2_GetActorLocation`))
  (bind _capsuleradius (`self.CapsuleRadius`))
  (bind _capsulehalfheight (`self.CapsuleHalfHeight`))
  (bind _returnvalue_2 (+ _returnvalue (`KismetMathLibrary.MakeVector` 0.0 0.0 _capsulehalfheight)))
  (bind (_returnvalue_x _returnvalue_y) (`KismetMathLibrary.BreakVector` (* (`PawnMovementComponent.GetLastInputVector` (`self.CharacterMovement`)) (* (`KismetMathLibrary.DegTan` (`local.CapsuleTiltAngle`)) _capsulehalfheight))))
  (bind _returnvalue_3 (+ _returnvalue (`KismetMathLibrary.MakeVector` _returnvalue_x _returnvalue_y _capsulehalfheight)))
  (bind (_outhit _returnvalue_4) (`KismetSystemLibrary.SphereTraceSingle` :`Start` _returnvalue_3 :`End` _returnvalue_3 :`Radius` _capsuleradius :`TraceChannel` "TraceTypeQuery1" :`DrawDebugType` "ForDuration"))
  (bind (_outhit_2 _returnvalue_5) (`KismetSystemLibrary.SphereTraceSingle` :`Start` _returnvalue_2 :`End` _returnvalue_2 :`Radius` _capsuleradius :`TraceChannel` "TraceTypeQuery1" :`DrawDebugType` "ForDuration"))
  (return (`KismetMathLibrary.BooleanNOR` _returnvalue_4 _returnvalue_5)))

(fn `CapsuleSetup`
  (`CapsuleComponent.SetCapsuleHalfHeight` (`self.CapsuleComponent`) (`self.CapsuleHalfHeight`) true))

(fn `CharacterMovementSetup`
  (bind _charactermovement (`self.CharacterMovement`))
  (set `CharacterMovementComponent.MaxWalkSpeed` (`self.MaxWalkSpeed`) _charactermovement)
  (set `CharacterMovementComponent.BrakingDecelerationWalking` (`self.BrakingDecelerationWalking`) _charactermovement)
  (set `CharacterMovementComponent.GroundFriction` (`self.GroundFriction`) _charactermovement))

(fn `GetAbilitySystemComponent`
  (returns (AbilitySystemComponent :type "/Game/Sotu/Blueprints/GAS/BPC_AbilitySystemComponent Object Reference"))
  (return (`self.BPC_AbilitySystemComponent`)))

(fn `IsInfiniteSlide`
  (returns (Result :type Boolean))
  (bind _returnvalue (`KismetMathLibrary.DegAcos` (`KismetMathLibrary.Dot_VectorVector` (`.Normal` (`GameplayStatics.BreakHitResult` (`.HitResult` (break `FindFloorResult` (`CharacterMovementComponent.CurrentFloor` (`self.CharacterMovement`)))))) (`SceneComponent.GetForwardVector` (`self.CapsuleComponent`)))))
  (return (and (> _returnvalue 0.0) (< _returnvalue 88.0))))

(fn `UserConstructionScript`)