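; Base character that implements walk, sprint, crouch, slide and jump using MovementData tuning, plus GAS interaction and component getters.
; Timelines animate capsule height and slide speed, holding full slide speed while a floor-slope check passes.
; Per-frame timers run stand-clearance traces and speed checks, setting loose gameplay tags alongside an in-air tag; the cannot-stand tag blocks uncrouching.
; Vaulting is only partial: a ledge-finding helper exists, but StartVault just traces.
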(event `self.K2_OnMovementModeChanged`
  (params (PrevMovementMode :type "EMovementMode Enum" :default "MOVE_None") (NewMovementMode :type "EMovementMode Enum" :default "MOVE_None") (PrevCustomMode :type Byte) (NewCustomMode :type Byte))
  (if (`|EnumEquality` NewMovementMode "MOVE_Falling")
    (`/Game/Sotu/Blueprints/BPFL_Sotu.AddLooseGameplayTag` self (`self.ContextInAirTag`))))

(event `self.ReceiveBeginPlay`
  (add `SotuAbilitySystemComponent.OnAttributeChanged` (`self.BPC_AbilitySystemComponent`) (delegate `Event_OnAttributeChanged`))
  (`self.SetupCapsuleComponent`)
  (`self.SetupCharacterMovement`))

(event `Event_OnAttributeChanged`
  (params (Attribute :type "GameplayAttribute Structure") (OldValue :type "Float (single-precision)") (NewValue :type "Float (single-precision)")))

(event `self.OnLanded`
  (params (Hit :type "HitResult Structure (by ref)"))
  (`/Game/Sotu/Blueprints/BPFL_Sotu.RemoveLooseGameplayTag` self (`self.ContextInAirTag`)))

(event `/Game/Sotu/Blueprints/Movement/BPI_MovementInterface.StartSprint`
  (set `CharacterMovementComponent.MaxWalkSpeed` (`/Game/Sotu/Blueprints/Movement/BP_MovementData.MaxSprintSpeed` (`self.MovementData`)) (`self.CharacterMovement`)))

(event `/Game/Sotu/Blueprints/Movement/BPI_MovementInterface.StartSlide`
  (bind _movementdata (`self.MovementData`))
  (bind _charactermovement (`self.CharacterMovement`))
  (set `CharacterMovementComponent.MaxWalkSpeed` (`/Game/Sotu/Blueprints/Movement/BP_MovementData.MaxSlideSpeed` _movementdata) _charactermovement)
  (set `CharacterMovementComponent.BrakingDecelerationWalking` (`/Game/Sotu/Blueprints/Movement/BP_MovementData.SlideBrakingDecelerationWalking` _movementdata) _charactermovement)
  (set `CharacterMovementComponent.GroundFriction` (`/Game/Sotu/Blueprints/Movement/BP_MovementData.SlideGroundFriction` _movementdata) _charactermovement)
  (`self.StartSlide_Anim`))

(event `/Game/Sotu/Blueprints/Movement/BPI_MovementInterface.StartJump`
  (`self.Jump`))

(event `/Game/Sotu/Blueprints/Movement/BPI_MovementInterface.StartVault`
  (`KismetSystemLibrary.SphereTraceSingle` (`self.K2_GetActorLocation`) (0.0 0.0 0.0) 0.0 "TraceTypeQuery1"))

(event `/Game/Sotu/Blueprints/Movement/BPI_MovementInterface.StartWalk`
  (set `CharacterMovementComponent.MaxWalkSpeed` (`/Game/Sotu/Blueprints/Movement/BP_MovementData.MaxWalkSpeed` (`self.MovementData`)) (`self.CharacterMovement`)))

(event `/Game/Sotu/Blueprints/Movement/BPI_MovementInterface.StartCrouch`
  (set `CharacterMovementComponent.MaxWalkSpeed` (`/Game/Sotu/Blueprints/Movement/BP_MovementData.MaxCrouchSpeed` (`self.MovementData`)) (`self.CharacterMovement`))
  (`self.StartCrouch_Anim`))

(event `/Game/Sotu/Blueprints/Movement/BPI_MovementInterface.EndSlide`
  (bind _charactermovement (`self.CharacterMovement`))
  (bind _movementdata (`self.MovementData`))
  (set `CharacterMovementComponent.BrakingDecelerationWalking` (`/Game/Sotu/Blueprints/Movement/BP_MovementData.BrakingDecelerationWalking` _movementdata) _charactermovement)
  (set `CharacterMovementComponent.GroundFriction` (`/Game/Sotu/Blueprints/Movement/BP_MovementData.GroundFriction` _movementdata) _charactermovement)
  (`self.EndSlide_Anim`))

(event `/Game/Sotu/Blueprints/Movement/BPI_MovementInterface.EndJump`
  (`self.StopJumping`))

(event `/Game/Sotu/Blueprints/Movement/BPI_MovementInterface.EndVault`)

(event `/Game/Sotu/Blueprints/Movement/BPI_MovementInterface.EndWalk`)

(event `/Game/Sotu/Blueprints/Movement/BPI_MovementInterface.EndSprint`)

(event `/Game/Sotu/Blueprints/Movement/BPI_MovementInterface.EndCrouch`
  (`self.EndCrouch_Anim`))

(event `StartCrouch_Anim`
  (bind _crouchtimeline (`self.CrouchTimeline`))
  (`TimelineComponent.SetPlayRate` _crouchtimeline (/ (`TimelineComponent.GetTimelineLength` _crouchtimeline) (`/Game/Sotu/Blueprints/Movement/BP_MovementData.CrouchDuration` (`self.MovementData`))))
  (`self.StartTimer_CanStand`)
  (bind (_direction _alpha) (`Timeline|CrouchTimeline` :!label _label)
    (:`Update`
      (`self.CrouchAnimUpdate` _direction _alpha))))

(event `StartSlide_Anim`
  (`TimelineComponent.SetPlayRate` (`self.SlideTimeline`) (/ (`TimelineComponent.GetTimelineLength` (`self.SlideTimeline`)) (`/Game/Sotu/Blueprints/Movement/BP_MovementData.SlideDuration` (`self.MovementData`))))
  (`self.StartCrouch_Anim`)
  (`self.StartTimer_StateSlide`)
  (bind (_direction _alpha) (`Timeline|SlideTimeline` :!via `PlayFromStart` :!label _label_2)
    (:`Update`
      (`self.SlideAnimUpdate` _alpha))))

(event `EndCrouch_Anim`
  (`self.EndTimer_CanStand`)
  (goto _label :!via `Reverse`))

(event `EndSlide_Anim`
  (`self.EndCrouch_Anim`)
  (`self.EndTimer_StateSlide`)
  (goto _label_2 :!via `Stop`))

(event `StartTimer_CanStand`
  (bind _returnvalue (`KismetSystemLibrary.K2_SetTimerDelegate` (delegate `Event_CanStand`) (`GameplayStatics.GetWorldDeltaSeconds`) true true))
  (set `self.CanStandTimerHandle` _returnvalue))

(event `StartTimer_StateSlide`
  (bind _returnvalue (`KismetSystemLibrary.K2_SetTimerDelegate` (delegate `Event_StateSlide`) (`GameplayStatics.GetWorldDeltaSeconds`) true true))
  (set `self.StateSlideTimerHandle` _returnvalue))

(event `Event_CanStand`
  (bind _contextcannotstandtag (`self.ContextCannotStandTag`))
  (if (`self.CanStand`)
    (`/Game/Sotu/Blueprints/BPFL_Sotu.RemoveLooseGameplayTag` self _contextcannotstandtag)
    (else
      (`/Game/Sotu/Blueprints/BPFL_Sotu.AddLooseGameplayTag` self _contextcannotstandtag))))

(event `Event_StateSlide`
  (bind _contextcannotslidetag (`self.ContextCannotSlideTag`))
  (if (> (`KismetMathLibrary.VSize` (`self.GetVelocity`)) (`/Game/Sotu/Blueprints/Movement/BP_MovementData.MaxCrouchSpeed` (`self.MovementData`)))
    (`/Game/Sotu/Blueprints/BPFL_Sotu.RemoveLooseGameplayTag` self _contextcannotslidetag)
    (else
      (`/Game/Sotu/Blueprints/BPFL_Sotu.AddLooseGameplayTag` self _contextcannotslidetag))))

(event `EndTimer_CanStand`
  (`KismetSystemLibrary.K2_ClearAndInvalidateTimerHandle` (`self.CanStandTimerHandle`)))

(event `EndTimer_StateSlide`
  (`KismetSystemLibrary.K2_ClearAndInvalidateTimerHandle` (`self.StateSlideTimerHandle`))
  (`/Game/Sotu/Blueprints/BPFL_Sotu.RemoveLooseGameplayTag` self (`self.ContextCannotSlideTag`)))

(fn `CanStand`
  (returns (Result :type Boolean))
  (locals (TraceStart :type "Vector Structure") (UpTraceResult :type Boolean) (UpForwardTraceResult :type Boolean) (ForwardTraceResult :type Boolean))
  (bind _movementdata (`self.MovementData`))
  (bind _movementdata_2 (`self.MovementData`))
  (bind _movementdata_3 (`self.MovementData`))
  (bind _capsulehalfheight (`/Game/Sotu/Blueprints/Movement/BP_MovementData.CapsuleHalfHeight` _movementdata))
  (bind _returnvalue (+ (`local.TraceStart`) (`KismetMathLibrary.MakeVector` 0.0 0.0 (`/Game/Sotu/Blueprints/Movement/BP_MovementData.CapsuleHalfHeight` _movementdata_3))))
  (bind (_returnvalue_x _returnvalue_y) (`KismetMathLibrary.BreakVector` (* (`PawnMovementComponent.GetLastInputVector` (`self.CharacterMovement`)) (* (`KismetMathLibrary.DegTan` (`/Game/Sotu/Blueprints/Movement/BP_MovementData.CanStandCapsuleTiltAngle` _movementdata)) _capsulehalfheight))))
  (bind (_returnvalue_x_2 _returnvalue_y_2) (`KismetMathLibrary.BreakVector` (* (`PawnMovementComponent.GetLastInputVector` (`self.CharacterMovement`)) (* (`KismetMathLibrary.DegTan` (`/Game/Sotu/Blueprints/Movement/BP_MovementData.CanStandCapsuleTiltAngle` _movementdata_2)) (`/Game/Sotu/Blueprints/Movement/BP_MovementData.CapsuleHalfHeight` _movementdata_2)))))
  (bind _returnvalue_2 (+ (`local.TraceStart`) (`KismetMathLibrary.MakeVector` _returnvalue_x_2 _returnvalue_y_2)))
  (bind _returnvalue_3 (+ (`local.TraceStart`) (`KismetMathLibrary.MakeVector` _returnvalue_x _returnvalue_y _capsulehalfheight)))
  (set `local.TraceStart` (+ (- (`self.K2_GetActorLocation`) (`KismetMathLibrary.MakeVector` 0.0 0.0 (`CapsuleComponent.GetScaledCapsuleHalfHeight` (`self.CapsuleComponent`)))) (`KismetMathLibrary.MakeVector` 0.0 0.0 (`/Game/Sotu/Blueprints/Movement/BP_MovementData.CapsuleHalfHeight` (`self.MovementData`)))))
  ; Up Trace
  (bind (_outhit _returnvalue_4) (`KismetSystemLibrary.SphereTraceSingle` :`Start` _returnvalue :`End` _returnvalue :`Radius` (`/Game/Sotu/Blueprints/Movement/BP_MovementData.CanStandSphereTraceRadius` _movementdata_3) :`TraceChannel` "TraceTypeQuery1" :`DrawDebugType` "ForOneFrame" :`TraceColor` (struct :`G` 1.0 :`B` 0.059422 :`A` 1.0)))
  (set `local.UpTraceResult` _returnvalue_4)
  ; Up Forward Trace
  (bind (_outhit_2 _returnvalue_5) (`KismetSystemLibrary.SphereTraceSingle` :`Start` _returnvalue_3 :`End` _returnvalue_3 :`Radius` (`/Game/Sotu/Blueprints/Movement/BP_MovementData.CanStandSphereTraceRadius` _movementdata) :`TraceChannel` "TraceTypeQuery1" :`DrawDebugType` "ForOneFrame" :`TraceColor` (struct :`R` 0.017489 :`G` 0.077913 :`B` 1.0 :`A` 1.0)))
  (set `local.UpForwardTraceResult` _returnvalue_5)
  ; Forward Trace
  (bind (_outhit_3 _returnvalue_6) (`KismetSystemLibrary.SphereTraceSingle` :`Start` _returnvalue_2 :`End` _returnvalue_2 :`Radius` (`/Game/Sotu/Blueprints/Movement/BP_MovementData.CanStandSphereTraceRadius` _movementdata_2) :`TraceChannel` "TraceTypeQuery1" :`DrawDebugType` "ForOneFrame"))
  (set `local.ForwardTraceResult` _returnvalue_6)
  (return (and (not (`local.UpTraceResult`)) (or (`local.ForwardTraceResult`) (not (`local.UpForwardTraceResult`))))))

(fn `CrouchAnimUpdate`
  (params (Selection :type "ETimelineDirection Enum" :default "Forward") (Alpha :type "Float (double-precision)"))
  (bind _movementdata (`self.MovementData`))
  (switch `ETimelineDirection` Selection
    (:`Forward`
      (`CapsuleComponent.SetCapsuleHalfHeight` (`self.CapsuleComponent`) (`KismetMathLibrary.Lerp` (`/Game/Sotu/Blueprints/Movement/BP_MovementData.CapsuleHalfHeight` _movementdata) (`/Game/Sotu/Blueprints/Movement/BP_MovementData.CrouchHalfHeight` _movementdata) Alpha) true :!label _label))
    (:`Backward`
      (if (not (`GameplayTagAssetInterface.HasMatchingGameplayTag` (`self.BPC_AbilitySystemComponent`) (`self.ContextCannotStandTag`)))
        (goto _label)))))

(fn `FindVaultEndLocation`
  (returns (Result :type Boolean) (Location :type "Vector Structure"))
  (locals (bFrontTraceResult :type Boolean :default false) (bDownTraceResult :type Boolean :default false))
  (bind _movementdata (`self.MovementData`))
  (bind _movementdata_2 (`self.MovementData`))
  (bind _returnvalue (and (`local.bFrontTraceResult`) (`local.bDownTraceResult`)))
  (bind _vaultminheight (`/Game/Sotu/Blueprints/Movement/BP_MovementData.VaultMinHeight` _movementdata))
  (bind (_returnvalue_x _returnvalue_y) (`KismetMathLibrary.BreakVector` (* (`self.GetActorForwardVector`) (`/Game/Sotu/Blueprints/Movement/BP_MovementData.VaultMaxDistance` _movementdata_2))))
  (bind (_returnvalue_x_2 _returnvalue_y_2) (`KismetMathLibrary.BreakVector` (* (`self.GetActorForwardVector`) (`/Game/Sotu/Blueprints/Movement/BP_MovementData.VaultWallOffset` _movementdata))))
  (bind _returnvalue_2 (+ (- (`self.K2_GetActorLocation`) (`KismetMathLibrary.MakeVector` 0.0 0.0 (`CapsuleComponent.GetScaledCapsuleHalfHeight` (`self.CapsuleComponent`)))) (`KismetMathLibrary.MakeVector` 0.0 0.0 (`/Game/Sotu/Blueprints/Movement/BP_MovementData.VaultMinHeight` _movementdata_2))))
  (bind (_outhit _returnvalue_3) (`KismetSystemLibrary.LineTraceSingle` :`Start` _returnvalue_2 :`End` (+ _returnvalue_2 (`KismetMathLibrary.MakeVector` _returnvalue_x _returnvalue_y)) :`TraceChannel` "TraceTypeQuery1" :`DrawDebugType` "Persistent"))
  (set `local.bFrontTraceResult` _returnvalue_3)
  (bind _returnvalue_4 (- (`.ImpactPoint` (`GameplayStatics.BreakHitResult` _outhit)) (`KismetMathLibrary.MakeVector` 0.0 0.0 _vaultminheight)))
  (bind _outhit_2 (`KismetSystemLibrary.LineTraceSingle` :`Start` (+ _returnvalue_4 (`KismetMathLibrary.MakeVector` _returnvalue_x_2 _returnvalue_y_2 (`/Game/Sotu/Blueprints/Movement/BP_MovementData.VaultMaxHeight` _movementdata))) :`End` (+ _returnvalue_4 (`KismetMathLibrary.MakeVector` _returnvalue_x_2 _returnvalue_y_2 _vaultminheight)) :`TraceChannel` "TraceTypeQuery1" :`DrawDebugType` "Persistent"))
  (bind (_bblockinghit _binitialoverlap _time _distance _location _impactpoint) (`GameplayStatics.BreakHitResult` _outhit_2))
  (set `local.bDownTraceResult` (not (== _distance 0.0)))
  (return _returnvalue (`KismetMathLibrary.SelectVector` _impactpoint (0.0 0.0 0.0) _returnvalue)))

(fn `GetAbilitySystemComponent`
  (returns (AbilitySystemComponent :type "/Game/Sotu/Blueprints/GAS/BPC_AbilitySystemComponent Object Reference"))
  (return (`self.BPC_AbilitySystemComponent`)))

(fn `GetMovementData`
  (returns (MovementData :type "/Game/Sotu/Blueprints/Movement/BP_MovementData Object Reference"))
  (return (`self.MovementData`)))

(fn `GetMovementManagerComponent`
  (returns (MovementManager :type "/Game/Sotu/Blueprints/Movement/BPC_MovementManagerComponent Object Reference"))
  (return (`self.BPC_MovemenManagerComponent`)))

(fn `GetWeaponComponent`
  (returns (WeaponComponent :type "/Game/Sotu/Blueprints/Weapon/BPC_WeaponComponent Object Reference"))
  (return (`self.BPC_WeaponComponent`)))

(fn `GetWeaponHandler`
  (returns (WeaponHandler :type "SkeletalMeshComponent Object Reference"))
  (return (`self.Mesh`)))

(fn `InteractLogic`
  (`AbilitySystemComponent.TryActivateAbilitiesByTag` (`self.BPC_AbilitySystemComponent`) (`BlueprintGameplayTagLibrary.MakeGameplayTagContainerFromTag` (`self.InteractTag`)) true)
  (`AbilitySystemBlueprintLibrary.SendGameplayEventToActor` self (`self.InteractTag`) (make `GameplayEventData` (struct) null null null null (struct) (struct) (struct) (`self.InteractDistance`))))

(fn `IsInfiniteSlide`
  (returns (Result :type Boolean))
  (bind _returnvalue (`KismetMathLibrary.DegAcos` (`KismetMathLibrary.Dot_VectorVector` (`.Normal` (`GameplayStatics.BreakHitResult` (`.HitResult` (break `FindFloorResult` (`CharacterMovementComponent.CurrentFloor` (`self.CharacterMovement`)))))) (`SceneComponent.GetForwardVector` (`self.CapsuleComponent`)))))
  (return (and (> _returnvalue 0.0) (< _returnvalue 88.0))))

(fn `SetupCapsuleComponent`
  (`CapsuleComponent.SetCapsuleHalfHeight` (`self.CapsuleComponent`) (`/Game/Sotu/Blueprints/Movement/BP_MovementData.CapsuleHalfHeight` (`self.MovementData`)) true))

(fn `SetupCharacterMovement`
  (bind _movementdata (`self.MovementData`))
  (bind _charactermovement (`self.CharacterMovement`))
  (set `CharacterMovementComponent.BrakingDecelerationWalking` (`/Game/Sotu/Blueprints/Movement/BP_MovementData.BrakingDecelerationWalking` _movementdata) _charactermovement)
  (set `CharacterMovementComponent.GroundFriction` (`/Game/Sotu/Blueprints/Movement/BP_MovementData.GroundFriction` _movementdata) _charactermovement))

(fn `SlideAnimUpdate`
  (params (Alpha :type "Float (double-precision)"))
  (bind _result (`self.IsInfiniteSlide`))
  (bind _movementdata (`self.MovementData`))
  (bind _charactermovement (`self.CharacterMovement`))
  (bind _maxslidespeed (`/Game/Sotu/Blueprints/Movement/BP_MovementData.MaxSlideSpeed` _movementdata))
  (`TimelineComponent.SetLooping` (`self.SlideTimeline`) _result)
  (if (not _result)
    (set `CharacterMovementComponent.MaxWalkSpeed` (`KismetMathLibrary.Lerp` (`/Game/Sotu/Blueprints/Movement/BP_MovementData.MaxCrouchSpeed` _movementdata) _maxslidespeed Alpha) _charactermovement)
    (else
      (`TimelineComponent.SetPlaybackPosition` (`self.SlideTimeline`) 0.0 false false)
      (set `CharacterMovementComponent.MaxWalkSpeed` _maxslidespeed _charactermovement))))

(fn `UserConstructionScript`)