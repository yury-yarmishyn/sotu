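; BPC_ObjectPoolComponent is an actor component that keeps a pool of spawned actors whose classes implement BPI_ObjectPool.
; SpawnObjectFromPool spawns such an actor, marks it not in use through SetInUseMessage and adds it to PooledObjects.
; FindFirstAvailableObjectFromPool returns the first pooled actor of the exact requested class implementing the interface, without checking its in-use state.
; BeginPlay is empty, and the event graph's spawn call is unconnected.
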(event `self.ReceiveBeginPlay`)

(fn `FindFirstAvailableObjectFromPool`
  (params (ObjectClass :type "Actor Class Reference"))
  (returns (Object :type "Actor Object Reference"))
  (for _array_element (`self.PooledObjects`)
    (if (and (== ObjectClass (`GameplayStatics.GetObjectClass` _array_element)) (`KismetSystemLibrary.DoesImplementInterface` _array_element "/Game/Sotu/Blueprints/ObjectPool/BPI_ObjectPool.BPI_ObjectPool_C"))
      (return _array_element))))

(fn `SpawnObjectFromPool`
  (params (Object :type "Actor Class Reference"))
  (if (`KismetSystemLibrary.DoesClassImplementInterface` Object "/Game/Sotu/Blueprints/ObjectPool/BPI_ObjectPool.BPI_ObjectPool_C")
    (bind _returnvalue (`|SpawnActorFromClass` Object (`KismetMathLibrary.MakeTransform` (0.0 0.0 0.0)) "Undefined" "MultiplyWithRoot" null null))
    (message `/Game/Sotu/Blueprints/ObjectPool/BPI_ObjectPool.SetInUse` _returnvalue false)
    (`KismetArrayLibrary.Array_Add` (`self.PooledObjects`) _returnvalue)))