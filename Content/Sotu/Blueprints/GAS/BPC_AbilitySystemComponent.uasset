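; Ability System Component that sets up its owner's GAS attributes and abilities on BeginPlay from InitData.
; Starting attribute values are applied through a single init Gameplay Effect, using each attribute's tag as a SetByCaller magnitude key.
; Abilities are granted at level 0, with their array index as InputID.
; An attribute-to-tag map provides lookups in both directions between attributes and Gameplay Tags.
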(event `self.ReceiveBeginPlay`
  (bind _initdata (`self.InitData`))
  (`self.InitializeAbilitySystem`)
  (`self.InitializeAttributeSet`)
  (`self.InitializeAttributes` (`/Game/Sotu/Blueprints/GAS/BP_InitData.AttributeData` _initdata))
  (`self.InitializeAbilities` (`/Game/Sotu/Blueprints/GAS/BP_InitData.AbilityData` _initdata)))

(fn `GetAttributeByTag`
  (params (GameplayTag :type "GameplayTag Structure"))
  (returns (Attribute :type "GameplayAttribute Structure"))
  (bind _attrubutestotags (`self.AttrubutesToTags`))
  (`/Engine/EditorBlueprintResources/StandardMacros.IsValid` _attrubutestotags
    (:`Is Valid`
      (bind (_keypin _valuepin) (`|MapForEach` (`/Game/Sotu/Blueprints/GAS/BP_AttributesToTags.AttributesToTags` _attrubutestotags))
        (:`then`
          (if (== GameplayTag _valuepin)
            (return _keypin)))))))

(fn `GetAttributeTag`
  (params (Attribute :type "GameplayAttribute Structure"))
  (returns (GameplayTag :type "GameplayTag Structure"))
  (bind _attrubutestotags (`self.AttrubutesToTags`))
  (`/Engine/EditorBlueprintResources/StandardMacros.IsValid` _attrubutestotags
    (:`Is Valid`
      (return (`BlueprintMapLibrary.Map_Find` (`/Game/Sotu/Blueprints/GAS/BP_AttributesToTags.AttributesToTags` _attrubutestotags) Attribute)))))

(fn `InitializeAbilities`
  (params (AbilityData :type "Array of GameplayAbility Class Reference"))
  (for (_array_element _array_index) AbilityData
    (`self.K2_GiveAbility` _array_element 0 _array_index)))

(fn `InitializeAttributes`
  (params (AttributeData :type "Map of GameplayAttribute Structure to Float (double-precision)"))
  (locals (EffectSpec :type "GameplayEffectSpecHandle Structure"))
  (bind _returnvalue (`self.GetOwner`))
  (if (`BlueprintMapLibrary.Map_IsNotEmpty` AttributeData)
    (bind _returnvalue_2 (`AbilitySystemBlueprintLibrary.MakeSpecHandleByClass` (`self.InitAttributesEffect`) _returnvalue _returnvalue))
    (set `local.EffectSpec` _returnvalue_2)
    (for _array_element (`self.GetAllAttributes`)
      (`AbilitySystemBlueprintLibrary.AssignTagSetByCallerMagnitude` (`local.EffectSpec`) (`self.GetAttributeTag` _array_element) (`BlueprintMapLibrary.Map_Find` AttributeData _array_element)))
    (`self.BP_ApplyGameplayEffectSpecToSelf` (`local.EffectSpec`))))