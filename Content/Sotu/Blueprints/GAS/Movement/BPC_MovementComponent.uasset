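; Movement component that acts as a tag-driven state machine on the Gameplay Ability System, starting its owner in walk.
; RecalculateMovementState reads the current State.Movement tag from the ability system, defaulting to Walking.
; It takes the first matching MovementTransitions data table row whose required and excluded tag conditions pass.
; The target state activates the matching walk, crouch, slide or sprint ability.
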(event `self.ReceiveBeginPlay`
  (bind _abilitysystemcomponent (message `/Game/Sotu/Blueprints/GAS/BPI_AbilitySystemComponent.GetAbilitySystemComponent` (`self.GetOwner`)))
  (bind _output_get (set `self.AbilitySystemComponentREF` _abilitysystemcomponent))
  (`AbilitySystemComponent.TryActivateAbilityByClass` _output_get "/Game/Sotu/Blueprints/GAS/GameplayAbilities/GA_Walk.GA_Walk_C" true))

(fn `FindDesiredMovementState`
  (params (FromMovementState :type "GameplayTag Structure (by ref)"))
  (returns (DesiredMovementState :type "GameplayTag Structure"))
  (bind _movementtransitions (`self.MovementTransitions`))
  (bind _abilitysystemcomponentref (`self.AbilitySystemComponentREF`))
  (bind _outrownames (`DataTableFunctionLibrary.GetDataTableRowNames` _movementtransitions))
  (for _array_element _outrownames
    (bind _returnvalue (`|GetDataTableRow` _movementtransitions _array_element)
      (:`then`
        (bind (_frommovementstate _conidionwithtags _conditionwithouttags _tomovementstate) (break `/Game/Sotu/Blueprints/GAS/Movement/S_MovementTransitions` _returnvalue))
        (if (== _frommovementstate (`local.FromMovementState`))
          (if (and (`GameplayTagAssetInterface.HasAllMatchingGameplayTags` _abilitysystemcomponentref _conidionwithtags) (or (not (`GameplayTagAssetInterface.HasAllMatchingGameplayTags` _abilitysystemcomponentref _conditionwithouttags)) (`KismetArrayLibrary.Array_IsEmpty` (`BlueprintGameplayTagLibrary.BreakGameplayTagContainer` _conditionwithouttags))))
            (return _tomovementstate)))))))

(fn `GetCurrentMovementState`
  (returns (ReturnValue :type "GameplayTag Structure"))
  (bind _output (`|GetArrayItem` (`BlueprintGameplayTagLibrary.BreakGameplayTagContainer` (`BlueprintGameplayTagLibrary.Filter` (`BlueprintGameplayTagLibrary.GetOwnedGameplayTags` (`self.AbilitySystemComponentREF`)) (`BlueprintGameplayTagLibrary.MakeGameplayTagContainerFromTag` (struct :`TagName` "State.Movement"))))))
  (if (`BlueprintGameplayTagLibrary.IsGameplayTagValid` _output)
    (return _output)
    (else
      (return (struct :`TagName` "State.Movement.Walking")))))

(fn `RecalculateMovementState`
  (bind _returnvalue (`self.GetCurrentMovementState`))
  (bind _desiredmovementstate (`self.FindDesiredMovementState` _returnvalue))
  (if (`BlueprintGameplayTagLibrary.IsGameplayTagValid` _desiredmovementstate)
    (`self.SetMovementState` _desiredmovementstate)))

(fn `SetMovementState`
  (params (ToMovementState :type "GameplayTag Structure"))
  (bind _abilitysystemcomponentref (`self.AbilitySystemComponentREF`))
  (`|SwitchGameplayTag` ToMovementState
    (:`State.Movement.Crouching`
      (`AbilitySystemComponent.TryActivateAbilityByClass` _abilitysystemcomponentref "/Game/Sotu/Blueprints/GAS/GameplayAbilities/GA_Crouch.GA_Crouch_C" true))
    (:`State.Movement.Sliding`
      (`AbilitySystemComponent.TryActivateAbilityByClass` _abilitysystemcomponentref "/Game/Sotu/Blueprints/GAS/GameplayAbilities/GA_Slide.GA_Slide_C" true))
    (:`State.Movement.Sprinting`
      (`AbilitySystemComponent.TryActivateAbilityByClass` _abilitysystemcomponentref "/Game/Sotu/Blueprints/GAS/GameplayAbilities/GA_Sprint.GA_Sprint_C" true))
    (:`State.Movement.Walking`
      (`AbilitySystemComponent.TryActivateAbilityByClass` _abilitysystemcomponentref "/Game/Sotu/Blueprints/GAS/GameplayAbilities/GA_Walk.GA_Walk_C" true))))