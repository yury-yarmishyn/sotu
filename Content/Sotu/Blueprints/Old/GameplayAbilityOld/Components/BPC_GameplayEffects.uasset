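; Gameplay effects component that applies data-driven effect objects to its owner and tracks the non-instant ones in a stack, printed every tick for debugging.
; Instant, duration and infinite applies share one path that checks required and blocked tags on the owner's gameplay state component, then constructs the effect class.
; Execution is a separate function that ApplyEffect never calls.
; Effect interactions are pass-through stubs, and max-stack validation is unwired.
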(event `self.ReceiveBeginPlay`
  (add `self.OnEffectApplied` (`|CreateDelegate` :!event `ExecuteEffect`)))

(event `self.ReceiveTick`
  (params (DeltaSeconds :type "Float (single-precision)"))
  (for _array_element (`self.EffectStack`)
    (`KismetSystemLibrary.PrintString` (`KismetSystemLibrary.GetDisplayName` _array_element) true true (struct :`G` 0.66 :`B` 1.0 :`A` 1.0) 0.0)))

(fn `AddEffectToStack`
  (params (Effect :type "/Game/Sotu/Blueprints/Old/GameplayAbilityOld/GameplayEffects/Effects/GE_Base Object Reference"))
  (if (`|EnumInequality` (`/Game/Sotu/Blueprints/Old/GameplayAbilityOld/GameplayEffects/EffectData/BP_EffectData.EffectType` (`/Game/Sotu/Blueprints/Old/GameplayAbilityOld/GameplayEffects/Effects/GE_Base.EffectData` Effect)) "NewEnumerator0")
    (`KismetArrayLibrary.Array_Add` (`self.EffectStack`) (`local.Effect`))))

(fn `ApplyDurationEffect`
  (params (EffectData :type "/Game/Sotu/Blueprints/Old/GameplayAbilityOld/GameplayEffects/EffectData/BP_DurationEffectData Object Reference"))
  (`self.ApplyEffect` EffectData))

(fn `ApplyEffect`
  (params (EffectData :type "/Game/Sotu/Blueprints/Old/GameplayAbilityOld/GameplayEffects/EffectData/BP_EffectData Object Reference"))
  (bind _result (`self.CanApplyEffect?` EffectData))
  (if _result
    (bind _returnvalue (`|GenericCreateObject` (`/Game/Sotu/Blueprints/Old/GameplayAbilityOld/GameplayEffects/EffectData/BP_EffectData.EffectClass` EffectData) EffectData))
    (`self.AddEffectToStack` _returnvalue)))

(fn `ApplyInfiniteEffect`
  (params (EffectData :type "/Game/Sotu/Blueprints/Old/GameplayAbilityOld/GameplayEffects/EffectData/BP_InfiniteEffectData Object Reference"))
  (`self.ApplyEffect` EffectData))

(fn `ApplyInstantEffect`
  (params (EffectData :type "/Game/Sotu/Blueprints/Old/GameplayAbilityOld/GameplayEffects/EffectData/BP_InstantEffectData Object Reference"))
  (`self.ApplyEffect` EffectData))

(fn `BlockedTagsValidation`
  (params (EffectData :type "/Game/Sotu/Blueprints/Old/GameplayAbilityOld/GameplayEffects/EffectData/BP_EffectData Object Reference"))
  (returns (Result :type Boolean))
  (bind _gameplaystatecomponent (message `/Game/Sotu/Blueprints/Old/GameplayAbilityOld/Interfaces/BPI_GameplayState.GetGameplayStateComponent` (`self.GetOwner`)))
  (return (not (`BlueprintGameplayTagLibrary.HasAnyTags` (`/Game/Sotu/Blueprints/Old/GameplayAbilityOld/Components/BPC_GameplayState.TagContainer` _gameplaystatecomponent) (`/Game/Sotu/Blueprints/Old/GameplayAbilityOld/GameplayEffects/EffectData/BP_EffectData.BlockedTags` EffectData)))))

(fn `CanApplyEffect?`
  (params (EffectData :type "/Game/Sotu/Blueprints/Old/GameplayAbilityOld/GameplayEffects/EffectData/BP_EffectData Object Reference"))
  (returns (Result :type Boolean))
  (`/Engine/EditorBlueprintResources/StandardMacros.IsValid` EffectData
    (:`Is Valid`
      (bind _result (`self.RequiredTagsValidation` EffectData))
      (bind _result_2 (`self.BlockedTagsValidation` EffectData))
      (return (and _result_2 _result)))
    (:`Is Not Valid`
      (return false))))

(fn `CancelEffect`
  (params (EffectData :type "/Game/Sotu/Blueprints/Old/GameplayAbilityOld/GameplayEffects/EffectData/BP_EffectData Object Reference"))
  (returns (UpdatedEffectData :type "/Game/Sotu/Blueprints/Old/GameplayAbilityOld/GameplayEffects/EffectData/BP_EffectData Object Reference"))
  (return EffectData))

(fn `ExecuteEffect`
  (params (EffectData :type "/Game/Sotu/Blueprints/Old/GameplayAbilityOld/GameplayEffects/EffectData/BP_EffectData Object Reference"))
  (bind _updatedeffectdata (`self.ExecuteEffectInteractions` EffectData))
  (bind _returnvalue (`|GenericCreateObject` (`/Game/Sotu/Blueprints/Old/GameplayAbilityOld/GameplayEffects/EffectData/BP_EffectData.EffectClass` EffectData) _updatedeffectdata))
  (`/Game/Sotu/Blueprints/Old/GameplayAbilityOld/GameplayEffects/Effects/GE_Base.ExecuteEffect` _returnvalue))

(fn `ExecuteEffectInteractions`
  (params (EffectData :type "/Game/Sotu/Blueprints/Old/GameplayAbilityOld/GameplayEffects/EffectData/BP_EffectData Object Reference"))
  (returns (UpdatedEffectData :type "/Game/Sotu/Blueprints/Old/GameplayAbilityOld/GameplayEffects/EffectData/BP_EffectData Object Reference"))
  (return EffectData))

(fn `ExecuteStackMultiply`)

(fn `GetEffectCount`
  (params (Effect :type "/Game/Sotu/Blueprints/Old/GameplayAbilityOld/GameplayEffects/Effects/GE_Base Object Reference"))
  (returns (EffectCount :type Integer))
  (locals (Temp :type Integer))
  (for _array_element (`self.EffectStack`)
    (if (== (`GameplayStatics.GetObjectClass` Effect) (`GameplayStatics.GetObjectClass` _array_element))
      (`/Engine/EditorBlueprintResources/StandardMacros.IncrementInt` (`local.Temp`))))
  (return (`local.Temp`)))

(fn `GetEffectFromStack`
  (params (EffectClass :type "/Game/Sotu/Blueprints/Old/GameplayAbilityOld/GameplayEffects/Effects/GE_Base Class Reference"))
  (returns (Effect :type "/Game/Sotu/Blueprints/Old/GameplayAbilityOld/GameplayEffects/Effects/GE_Base Object Reference"))
  (for _array_element (`self.EffectStack`)
    (if (== (`GameplayStatics.GetObjectClass` _array_element) EffectClass)
      (return _array_element)))
  (return null))

(fn `GetRelativeEffectIndex`
  (params (Effect :type "/Game/Sotu/Blueprints/Old/GameplayAbilityOld/GameplayEffects/Effects/GE_Base Object Reference"))
  (returns (Index :type Integer))
  (locals (CurrentIndex :type Integer))
  (for _array_element (`self.EffectStack`)
    (if (== (`GameplayStatics.GetObjectClass` Effect) (`GameplayStatics.GetObjectClass` _array_element))
      (bind _result (`/Engine/EditorBlueprintResources/StandardMacros.IncrementInt` (`local.CurrentIndex`))
        (:`  `
          (if (== Effect _array_element)
            (return _result))))))
  (return -1))

(fn `InvertEffect`
  (params (EffectData :type "/Game/Sotu/Blueprints/Old/GameplayAbilityOld/GameplayEffects/EffectData/BP_EffectData Object Reference"))
  (returns (UpdatedEffectData :type "/Game/Sotu/Blueprints/Old/GameplayAbilityOld/GameplayEffects/EffectData/BP_EffectData Object Reference"))
  (return EffectData))

(fn `MultiplyEffect`
  (params (EffectData :type "/Game/Sotu/Blueprints/Old/GameplayAbilityOld/GameplayEffects/EffectData/BP_EffectData Object Reference"))
  (returns (UpdatedEffectData :type "/Game/Sotu/Blueprints/Old/GameplayAbilityOld/GameplayEffects/EffectData/BP_EffectData Object Reference"))
  (return EffectData))

(fn `OverrideEffect`
  (params (EffectData :type "/Game/Sotu/Blueprints/Old/GameplayAbilityOld/GameplayEffects/EffectData/BP_EffectData Object Reference"))
  (returns (UpdatedEffectData :type "/Game/Sotu/Blueprints/Old/GameplayAbilityOld/GameplayEffects/EffectData/BP_EffectData Object Reference"))
  (return EffectData))

(fn `RemoveEffectFromStack`
  (params (EffectClass :type "/Game/Sotu/Blueprints/Old/GameplayAbilityOld/GameplayEffects/Effects/GE_Base Object Reference"))
  (`KismetArrayLibrary.Array_RemoveItem` (`self.EffectStack`) EffectClass))

(fn `RequiredTagsValidation`
  (params (EffectData :type "/Game/Sotu/Blueprints/Old/GameplayAbilityOld/GameplayEffects/EffectData/BP_EffectData Object Reference"))
  (returns (Result :type Boolean))
  (bind _gameplaystatecomponent (message `/Game/Sotu/Blueprints/Old/GameplayAbilityOld/Interfaces/BPI_GameplayState.GetGameplayStateComponent` (`self.GetOwner`)))
  (return (`BlueprintGameplayTagLibrary.HasAllTags` (`/Game/Sotu/Blueprints/Old/GameplayAbilityOld/Components/BPC_GameplayState.TagContainer` _gameplaystatecomponent) (`/Game/Sotu/Blueprints/Old/GameplayAbilityOld/GameplayEffects/EffectData/BP_EffectData.RequiredTags` EffectData))))

(fn `StackValidation`
  (params (EffectData :type "/Game/Sotu/Blueprints/Old/GameplayAbilityOld/GameplayEffects/EffectData/BP_EffectData Object Reference"))
  (returns (Result :type Boolean))
  (switch `/Game/Sotu/Blueprints/Old/GameplayAbilityOld/GameplayEffects/Enum/E_EffectType` (`/Game/Sotu/Blueprints/Old/GameplayAbilityOld/GameplayEffects/EffectData/BP_EffectData.EffectType` EffectData)
    (:`NewEnumerator0`
      (return true))))