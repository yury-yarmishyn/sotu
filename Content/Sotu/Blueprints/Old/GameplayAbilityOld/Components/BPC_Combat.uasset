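; Actor component for combat, an unfinished framework that runs attacks described by an AttackData input.
; Attack validates the data, checks the owner's gameplay state tags against TagsBlockAttack, then calls an empty PlayAttackAnim.
; GetAttackTargets dispatches each attack type to hit scan, projectile, sphere trace or melee functions, which are placeholders returning no hits.
; Target gathering, hit reactions and effect application are disconnected from Attack, and the latter two are empty stubs.
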(fn `ApplyEffects`
  (params (Targets :type "Array of Actor Object Reference")))

(fn `Attack`
  (params (AttackData :type "/Game/Sotu/Blueprints/Old/BP_AttackData Object Reference"))
  (bind _result (`self.CanAttack?` AttackData))
  (if _result
    (`self.PlayAttackAnim` AttackData)))

(fn `AttackHitScan`
  (params (AttackData :type "/Game/Sotu/Blueprints/Old/BP_AttackData Object Reference"))
  (returns (Targets :type "Array of Actor Object Reference"))
  (`KismetSystemLibrary.PrintString` "HitScan"))

(fn `AttackMelee`
  (params (AttackData :type "/Game/Sotu/Blueprints/Old/BP_AttackData Object Reference"))
  (returns (Targets :type "Array of Actor Object Reference"))
  (return))

(fn `AttackProjectile`
  (params (AttackData :type "/Game/Sotu/Blueprints/Old/BP_AttackData Object Reference"))
  (returns (Targets :type "Array of Actor Object Reference"))
  (`KismetSystemLibrary.PrintString` "Projectile"))

(fn `AttackSphereTrace`
  (params (AttackData :type "/Game/Sotu/Blueprints/Old/BP_AttackData Object Reference"))
  (returns (Targets :type "Array of Actor Object Reference"))
  (locals (TargetsMelee :type "Array of Actor Object Reference"))
  (`KismetSystemLibrary.PrintString` "Melee")
  (bind _outhits (`KismetSystemLibrary.SphereTraceMultiForObjects` (`Actor.K2_GetActorLocation` (`self.GetOwner`)) (0.0 0.0 0.0) 0.0 (`|MakeArray` "ObjectTypeQuery2" "ObjectTypeQuery3" :!type "EObjectTypeQuery Enum")))
  (for _array_element _outhits
    _))

(fn `CanAttack?`
  (params (AttackData :type "/Game/Sotu/Blueprints/Old/BP_AttackData Object Reference"))
  (returns (Result :type Boolean))
  (`/Engine/EditorBlueprintResources/StandardMacros.IsValid` AttackData
    (:`Is Valid`
      (bind _gameplaystatecomponent (message `/Game/Sotu/Blueprints/Old/GameplayAbilityOld/Interfaces/BPI_GameplayState.GetGameplayStateComponent` (`self.GetOwner`)))
      (bind _returnvalue (`BlueprintGameplayTagLibrary.HasAnyTags` (`/Game/Sotu/Blueprints/Old/GameplayAbilityOld/Components/BPC_GameplayState.TagContainer` _gameplaystatecomponent) (`self.TagsBlockAttack`)))
      (return (not _returnvalue)))
    (:`Is Not Valid`
      (return false))))

(fn `GetAttackTargets`
  (params (AttackData :type "/Game/Sotu/Blueprints/Old/BP_AttackData Object Reference"))
  (returns (Targets :type "Array of Actor Object Reference"))
  (locals (CurrentTargets :type "Array of Actor Object Reference"))
  (for _array_element (`.AttackTypeData_41_2D82A2984744C2C3785B1EA03D109ABA` (break `/Game/Sotu/Blueprints/Old/S_AttackData` (`/Game/Sotu/Blueprints/Old/BP_AttackData.AttackData` AttackData)))
    (bind _attacktype (`/Game/Sotu/Blueprints/Old/BP_AttackTypeData.AttackType` _array_element))
    (switch `/Game/Sotu/Blueprints/Old/E_AttackType` _attacktype
      (:`NewEnumerator0`
        (bind _targets (`self.AttackHitScan` AttackData)))
      (:`NewEnumerator1`
        (bind _targets_2 (`self.AttackProjectile` AttackData)))
      (:`NewEnumerator2`
        (bind _targets_3 (`self.AttackSphereTrace` AttackData)))
      (:`NewEnumerator3`
        (bind _targets_4 (`self.AttackMelee` AttackData))))
    (`KismetArrayLibrary.Array_Append` (`local.CurrentTargets`) (select `/Game/Sotu/Blueprints/Old/E_AttackType` _attacktype :`NewEnumerator0` _targets :`NewEnumerator1` _targets_2 :`NewEnumerator2` _targets_3 :`NewEnumerator3` _targets_4)))
  (return (`local.CurrentTargets`)))

(fn `PlayAttackAnim`
  (params (AttackData :type "/Game/Sotu/Blueprints/Old/BP_AttackData Object Reference")))

(fn `PlayHitReactionAnim`
  (params (Targets :type "Array of Actor Object Reference")))