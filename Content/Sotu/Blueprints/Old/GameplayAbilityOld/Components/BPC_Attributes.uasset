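; Attribute component that stores an owner's attribute values in a map keyed by attribute tag, within an older gameplay ability setup.
; On BeginPlay it fills the map from the base values in the AttributesData table, if one is valid.
; A getter reads values by tag, while the setter only updates tags already in the map and then calls OnAttributeChanged with the new value.
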(event `self.ReceiveBeginPlay`
  (`self.InitAttributes`))

(fn `GetAttributeValue`
  (params (AttributeTag :type "GameplayTag Structure"))
  (returns (AttributeValue :type "Float (double-precision)"))
  (return (`BlueprintMapLibrary.Map_Find` (`self.Attributes`) AttributeTag)))

(fn `InitAttributes`
  (bind _attributesdata (`self.AttributesData`))
  (`/Engine/EditorBlueprintResources/StandardMacros.IsValid` _attributesdata
    (:`Is Valid`
      (bind _outrownames (`DataTableFunctionLibrary.GetDataTableRowNames` _attributesdata))
      (for _array_element _outrownames
        (bind _returnvalue (`|GetDataTableRow` _attributesdata _array_element)
          (:`then`
            (bind (_attributetag _basevalue) (break `/Game/Sotu/Blueprints/Old/GameplayAbilityOld/Attributes/S_Attribute` _returnvalue))
            (`BlueprintMapLibrary.Map_Add` (`self.Attributes`) _attributetag _basevalue)))))))

(fn `SetAttributeValue`
  (params (AttributeTag :type "GameplayTag Structure") (NewValue :type "Float (double-precision)"))
  (bind _attributes (`self.Attributes`))
  (if (`.ReturnValue` (`BlueprintMapLibrary.Map_Find` _attributes AttributeTag))
    (`BlueprintMapLibrary.Map_Add` _attributes AttributeTag NewValue)
    (`self.OnAttributeChanged` AttributeTag NewValue)))