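; Dialogue component that runs a conversation on its owning actor through a Behavior Tree started on the owner's AI controller.
; On BeginPlay it caches the dialogue and replies widgets from the owner's widget components.
; The first interact starts the tree; later ones progress the typewriter text.
; Setter and clear functions drive dialogue text and reply list; EndDialogue is empty, and InDialogue is never reset here.
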(event `self.ReceiveBeginPlay`
  (`self.InitDialogueComponents`))

(fn `ClearDialogue`
  (`/Game/Sotu/Blueprints/Old/DialogueOld/WBP_Dialogue.ClearDialogue` (`self.DialogueREF`)))

(fn `ClearReplies`
  (`/Game/Sotu/Blueprints/Old/DialogueOld/WBP_Replies.RemoveAllItemsFromListView` (`self.RepliesREF`)))

(fn `EndDialogue`)

(fn `InitDialogueComponents`
  (bind _returnvalue (`self.GetOwner`))
  (`|ExecutionSequence`
    (:`then_0`
      (bind _dialoguewidget (message `/Game/Sotu/Blueprints/Interfaces/BPI_Dialogue.GetDialogueWidget` _returnvalue))
      (`/Engine/EditorBlueprintResources/StandardMacros.IsValid` _dialoguewidget
        (:`Is Valid`
          (bind _aswbp_dialogue (cast `/Game/Sotu/Blueprints/Old/DialogueOld/WBP_Dialogue` (`WidgetComponent.GetUserWidgetObject` _dialoguewidget)))
          (set `self.DialogueREF` _aswbp_dialogue))))
    (:`then_1`
      (bind _replieswidget (message `/Game/Sotu/Blueprints/Interfaces/BPI_Dialogue.GetRepliesWidget` _returnvalue))
      (`/Engine/EditorBlueprintResources/StandardMacros.IsValid` _replieswidget
        (:`Is Valid`
          (bind _aswbp_replies (cast `/Game/Sotu/Blueprints/Old/DialogueOld/WBP_Replies` (`WidgetComponent.GetUserWidgetObject` _replieswidget)))
          (set `self.RepliesREF` _aswbp_replies))))))

(fn `OnInteract`
  (if (`self.bInDialogue?`)
    (`/Game/Sotu/Blueprints/Old/DialogueOld/WBP_Dialogue.ProgressText` (`self.DialogueREF`))
    (else
      (`self.RunDialogueTree`)
      (set `self.bInDialogue?` true))))

(fn `RunDialogueTree`
  (bind _btasset (`self.BTAsset`))
  (`/Engine/EditorBlueprintResources/StandardMacros.IsValid` _btasset
    (:`Is Valid`
      (`AIController.RunBehaviorTree` (`AIBlueprintHelperLibrary.GetAIController` (`self.GetOwner`)) _btasset))))

(fn `SetDialogue`
  (params (DialogueText :type Text))
  (bind _dialogueref (`self.DialogueREF`))
  (`/Engine/EditorBlueprintResources/StandardMacros.IsValid` _dialogueref
    (:`Is Valid`
      (`/Game/Sotu/Blueprints/Old/DialogueOld/WBP_Dialogue.ClearDialogue` _dialogueref)
      (set `/Game/Sotu/Blueprints/Old/DialogueOld/WBP_Dialogue.DialogueText` DialogueText _dialogueref)
      (`/Game/Sotu/Blueprints/Old/DialogueOld/WBP_Dialogue.RunTypewriter` _dialogueref))))

(fn `SetReplies`
  (params (Options :type "Array of Text"))
  (bind _repliesref (`self.RepliesREF`))
  (`/Engine/EditorBlueprintResources/StandardMacros.IsValid` _repliesref
    (:`Is Valid`
      (for _array_element Options
        (`/Game/Sotu/Blueprints/Old/DialogueOld/WBP_Replies.AddItemToListView` _repliesref _array_element)))))