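; Weapon component that lets its owning actor equip a weapon and trigger its attacks.
; Equipping requires the class's default tag to be in the available weapons and no blocking tags on the owner's gameplay state component.
; The weapon spawns by setting the class on a child actor component fetched from the owner via message call.
; Attack and AlternativeAttack forward to that BP_WeaponBase actor, while UnequipWeapon is empty.
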(event `self.ReceiveBeginPlay`)

(fn `AlternativeAttack`
  (bind _weaponhandler (message `/Game/Sotu/Blueprints/Old/GameplayAbilityOld/Interfaces/BPI_Weapon.GetWeaponHandler` (`self.GetOwner`)))
  (bind _asbp_weapon_base (cast `/Game/Sotu/Blueprints/Weapons/BP_WeaponBase` (`ChildActorComponent.ChildActor` _weaponhandler)))
  (`/Game/Sotu/Blueprints/Weapons/BP_WeaponBase.AlternativeAttack` _asbp_weapon_base (`self.GetOwner`)))

(fn `Attack`
  (bind _weaponhandler (message `/Game/Sotu/Blueprints/Old/GameplayAbilityOld/Interfaces/BPI_Weapon.GetWeaponHandler` (`self.GetOwner`)))
  (bind _asbp_weapon_base (cast `/Game/Sotu/Blueprints/Weapons/BP_WeaponBase` (`ChildActorComponent.ChildActor` _weaponhandler)))
  (`/Game/Sotu/Blueprints/Weapons/BP_WeaponBase.Attack` _asbp_weapon_base (`self.GetOwner`)))

(fn `CanEquipWeapon?`
  (params (Weapon :type "/Game/Sotu/Blueprints/Weapons/BP_WeaponBase Class Reference"))
  (returns (Result :type Boolean))
  (if (`KismetSystemLibrary.IsValidClass` Weapon)
    (bind _returnvalue (`BlueprintGameplayTagLibrary.HasTag` (`self.AvailableWeapons`) (defaults `Object` Weapon)))
    (bind _gameplaystatecomponent (message `/Game/Sotu/Blueprints/Old/GameplayAbilityOld/Interfaces/BPI_GameplayState.GetGameplayStateComponent` (`self.GetOwner`)))
    (bind _returnvalue_2 (`BlueprintGameplayTagLibrary.HasAnyTags` (`/Game/Sotu/Blueprints/Old/GameplayAbilityOld/Components/BPC_GameplayState.TagContainer` _gameplaystatecomponent) (`self.TagsBlockEquip`)))
    (return (and (not _returnvalue_2) _returnvalue))
    (else
      (return false))))

(fn `EquipWeapon`
  (params (WeaponClass :type "/Game/Sotu/Blueprints/Weapons/BP_WeaponBase Class Reference"))
  (bind _result (`self.CanEquipWeapon?` WeaponClass))
  (if _result
    (bind _weaponhandler (message `/Game/Sotu/Blueprints/Old/GameplayAbilityOld/Interfaces/BPI_Weapon.GetWeaponHandler` (`self.GetOwner`)))
    (`ChildActorComponent.SetChildActorClass` _weaponhandler WeaponClass)))

(fn `UnequipWeapon`
  (params (Weapon :type "/Game/Sotu/Blueprints/Weapons/BP_WeaponBase Class Reference")))