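; GA_Slide is a Gameplay Ability that runs the player's slide, activating only while horizontal velocity is non-zero.
; Activation sends a start-slide message to the outer object, then listens for two tag changes.
; Removal of the crouch-held input tag or addition of the CannotSlide state tag ends the ability.
; Ending sends an end-slide message and has the movement manager recalculate movement state.
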(event `self.K2_ActivateAbility`
  (message `/Game/Sotu/Blueprints/Movement/BPI_MovementInterface.StartSlide` (`KismetSystemLibrary.GetOuterObject` self))
  (`AbilityTask_WaitGameplayTagRemoved.WaitGameplayTagRemove` (struct :`TagName` "Input.Crouch.Held") null
    (:`then`
      (`AbilityTask_WaitGameplayTagAdded.WaitGameplayTagAdd` (struct :`TagName` "State.Context.CannotSlide") null
        (:`Added`
          _)))
    (:`Removed`
      _))
  (`self.K2_EndAbility`))

(event `self.K2_OnEndAbility`
  (params (bWasCancelled :type Boolean))
  (bind _returnvalue (`KismetSystemLibrary.GetOuterObject` self))
  (message `/Game/Sotu/Blueprints/Movement/BPI_MovementInterface.EndSlide` _returnvalue)
  (bind _movementmanager (message `/Game/Sotu/Blueprints/Movement/BPI_MovementInterface.GetMovementManagerComponent` _returnvalue))
  (`/Game/Sotu/Blueprints/Movement/BPC_MovementManagerComponent.RecalculateMovementState` _movementmanager))

(fn `K2_CanActivateAbility`
  (params (ActorInfo :type "GameplayAbilityActorInfo Structure") (Handle :type "GameplayAbilitySpecHandle Structure"))
  (returns (RelevantTags :type "GameplayTagContainer Structure") (ReturnValue :type Boolean))
  (return (struct) (> (`KismetMathLibrary.VSizeXY` (`MovementComponent.Velocity` (`.MovementComponent` (break `GameplayAbilityActorInfo` ActorInfo)))) 0.0)))